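; BP_possible_Objective is a mission objective trigger with a marker, part of the mission system, that starts hidden with collision disabled.
; Its ActiveMission interface event enables the box collision and shows the marker when the passed mission differs from its Objective.
; When BP_ThirdPersonCharacter overlaps the box, it calls SildeOff on the character, plays an explosion sound and destroys itself, with no effective mission check.
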(event `self.ReceiveBeginPlay`
  (`PrimitiveComponent.SetCollisionEnabled` (`self.Box`) "NoCollision")
  (`SceneComponent.SetVisibility` (`self.MissionMarker`) false false))

(event `/Game/Mission_System/ActiveMission.ActiveMission`
  (params (ActiveMission :type String))
  ;[1 1 1] Interface
  (if (`KismetStringLibrary.NotEqual_StrStr` ActiveMission (`self.Objective`))
    (`PrimitiveComponent.SetCollisionEnabled` (`self.Box`) "QueryAndPhysics")
    (`SceneComponent.SetVisibility` (`self.MissionMarker`) true false)))

(event `self.Box.OnComponentBeginOverlap`
  (params (OverlappedComponent :type "PrimitiveComponent Object Reference") (OtherActor :type "Actor Object Reference") (OtherComp :type "PrimitiveComponent Object Reference") (OtherBodyIndex :type Integer) (bFromSweep :type Boolean) (SweepResult :type "HitResult Structure (by ref)"))
  (bind _asbp_third_person_character (cast `/Game/ThirdPerson/Blueprints/BP_ThirdPersonCharacter` OtherActor))
  (bind _output_get (set `self.As BP Third Person Character` _asbp_third_person_character))
  (if true
    (`/Game/ThirdPerson/Blueprints/BP_ThirdPersonCharacter.SildeOff` _output_get)
    (`GameplayStatics.PlaySound2D` "/Game/StarterContent/Audio/Explosion01.Explosion01" 1.0 1.0 0.0 null null)
    (`self.K2_DestroyActor`)))

(fn `UserConstructionScript`)